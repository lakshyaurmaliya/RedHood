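; BP_EnemyPatrol is an overlap-driven actor that controls the combat target of a group of enemies in its PatrolActors array.
; When an actor implementing BPI_RedHood begins overlapping it, every valid patrol actor receives that actor through SetCombatTargetMessage.
; When such an actor stops overlapping, the same message is sent without a target, clearing it for the whole group.
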(event Collision|EventActorBeginOverlap
  (params (OtherActor :type Actor%20Object%20Reference))
  (if (Utilities|DoesObjectImplementInterface OtherActor "/Game/Blueprints/Interfaces/BPI_RedHood.BPI_RedHood_C")
    (for _array_element (Variables|Default|GetPatrolActors)
      (Utilities|IsValid _array_element
        (:Is%20Valid
          (Class|BPIEnemy|SetCombatTarget(Message) _array_element OtherActor))))))

(event Collision|EventActorEndOverlap
  (params (OtherActor :type Actor%20Object%20Reference))
  (if (Utilities|DoesObjectImplementInterface OtherActor "/Game/Blueprints/Interfaces/BPI_RedHood.BPI_RedHood_C")
    (for _array_element (Variables|Default|GetPatrolActors)
      (Utilities|IsValid _array_element
        (:Is%20Valid
          (Class|BPIEnemy|SetCombatTarget(Message) _array_element))))))

(fn ConstructionScript)