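; Base enemy character that links combat events to its AI blackboard and overhead health bar widget.
; Blackboard keys hold the alive state and combat target, and SetHitReacting clears the hit-reacting flag.
; GetHit extends the parent's damage handling by updating the bar and, while that widget is valid, calling Die at zero health.
; Die clears the alive key, disables capsule collision, hides the bar and sets a short life span.
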(event EventSetHitReacting
  (params (IsHitReacting :type Boolean))
  (AI|Components|Blackboard|SetValueasBool (AI|GetBlackboard (Pawn|GetController)) (Variables|Default|GetHitReactingKeyName) false))

(event EventSetCombatTarget
  (params (CombatTarget :type Actor%20Object%20Reference))
  (AI|Components|Blackboard|SetValueasObject (AI|GetBlackboard (Pawn|GetController)) (Variables|Default|GetCombatTargetBBKeyName) CombatTarget))

(event EventAttack
  (CallFunction|PlayAttackAnim))

(event EventBeginPlay
  (|CallParentFunction)
  (bind _aswbp_enemy_health_bar (Utilities|Casting|CastToWBP_EnemyHealthBar (UserInterface|GetUserWidgetObject (Variables|Default|GetHealthBarWidget))))
  (Variables|Default|SetEnemyHealthBar _aswbp_enemy_health_bar)
  (AI|Components|Blackboard|SetValueasBool (AI|GetBlackboard (Pawn|GetController)) (Variables|Default|GetAliveBBKeyName) true))

(fn ConstructionScript)

(fn ChangeDirection
  (Transformation|SetActorRotation (Math|Rotator|CombineRotators (Transformation|GetActorRotation) "0.000000,180.000000,0.000000")))

(fn GetHit
  (params (InDamage :type Float%20%28double-precision%29))
  (|CallParentFunction InDamage)
  (bind _enemyhealthbar (Variables|Default|GetEnemyHealthBar)
    (:then
      (Default|SetHealthPercent _enemyhealthbar (Math|Float|SafeDivide (Variables|Default|GetHealth) (Variables|Default|GetMaxHealth)))
      (if (<= (Variables|Default|GetHealth) 0.0)
        (CallFunction|Die)))
    (:else)))

(fn Die
  (Utilities|FlowControl|Sequence
    (:then_0
      ;[0.15 0.15 0.15 0.5] Disable Behaviour Tree
      (AI|Components|Blackboard|SetValueasBool (AI|GetBlackboard (Pawn|GetController)) (Variables|Default|GetAliveBBKeyName) false))
    (:then_1
      ;[0.15 0.15 0.15 0.5] No Collision
      (Collision|SetCollisionEnabled (Variables|Default|GetCapsuleComponent) "NoCollision"))
    (:then_2
      ;[0.15 0.15 0.15 0.5] Hide Health Bar
      (Rendering|SetVisibility (Variables|Default|GetHealthBarWidget) false false))
    (:then_3
      ;[0.15 0.15 0.15 0.5] Set Life Span
      (Actor|SetLifeSpan 3.0))))